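; Player character that moves tile by tile on a GridNavMesh and carries and operates light items.
; Directional inputs turn the mesh and update a validated grid index, which Tick interpolates toward, accepting new moves only on arrival.
; Pick-or-drop attaches the current light item or drops it on the tile if unshared.
; Use switches a remote light off immediately but only flags switch-on, deferred to the beat; DamagePlayer is an empty stub.
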(event EventBeginPlay
  (bind _returnvalue (Actor|GetActorOfClass "/Game/Blueprints/GridNavMesh.GridNavMesh_C"))
  (bind _output_get (Variables|Default|SetGrid _returnvalue))
  (if (.IsValid (Default|GetGridIndexfromLocationNE _output_get (Transformation|GetActorLocation)))
    (bind _output_get_2 (Variables|Default|SetPlayerGridLoc (.Int%20Pt (Default|GetGridIndexfromLocationNE _output_get (Transformation|GetActorLocation)))))
    (CallFunction|SetTargetLocation _output_get_2)))

(event EventTick
  (params (DeltaSeconds :type Float%20%28single-precision%29))
  (bind _returnvalue (Transformation|GetActorLocation))
  (if (Utilities|Operators|EqualEqual (Variables|Default|GetTargetLocation) _returnvalue 1e+01)
    (Variables|Default|SetIsNotMoving true)
    (else
      (Transformation|SetActorLocation (Math|Interpolation|VInterpTo _returnvalue (Variables|Default|GetTargetLocation) DeltaSeconds (Variables|Default|GetMovementSpeed)) true false))))

(event Input|ActionEvents|InputActionForward
  (params (Key :type Key%20Structure :default "None"))
  (:Pressed
    (CallFunction|MovePlayer (Utilities|Struct|MakeIntPoint 0 1))
    (Transformation|SetRelativeRotation (Variables|Default|GetStaticMesh) "0, 0, 0" false false)))

(event Input|ActionEvents|InputActionBackward
  (params (Key :type Key%20Structure :default "None"))
  (:Pressed
    (CallFunction|MovePlayer (Utilities|Struct|MakeIntPoint 0 -1))
    (Transformation|SetRelativeRotation (Variables|Default|GetStaticMesh) "0,180.000000, 0" false false)))

(event Input|ActionEvents|InputActionRight
  (params (Key :type Key%20Structure :default "None"))
  (:Pressed
    (CallFunction|MovePlayer (Utilities|Struct|MakeIntPoint -1 0))
    (Transformation|SetRelativeRotation (Variables|Default|GetStaticMesh) "0,90.000000, 0" false false)))

(event Input|ActionEvents|InputActionLeft
  (params (Key :type Key%20Structure :default "None"))
  (:Pressed
    (CallFunction|MovePlayer (Utilities|Struct|MakeIntPoint 1 0))
    (Transformation|SetRelativeRotation (Variables|Default|GetStaticMesh) "0,-90.000000, 0" false false)))

(event Input|ActionEvents|InputActionPickOrDropItem
  (params (Key :type Key%20Structure :default "None"))
  (:Pressed
    (if (Variables|Default|GetItemEquipped)
      (CallFunction|DropItem)
      (else
        (CallFunction|PickUpItem)))))

(event Input|ActionEvents|InputActionUseItem
  (params (Key :type Key%20Structure :default "None"))
  (bind _newremotelightitem (Variables|Default|GetNewRemoteLightItem))
  ;[1 1 1] RC Light activated with each beat & not immediatly on player click
  (:Pressed
    (Utilities|IsValid _newremotelightitem
      (:Is%20Valid
        (if (Variables|/Game/Blueprints/Items/LightItemMaster.LightItemMaster_C|GetTurnedOnByPlayer _newremotelightitem)
          (Default|LightsOff _newremotelightitem)
          (Default|InstigatorTurnConnectedTilesOff _newremotelightitem)
          (Variables|/Game/Blueprints/Items/LightItemMaster.LightItemMaster_C|SetTurnedOnByPlayer _newremotelightitem false)
          (else
            (Variables|/Game/Blueprints/Items/LightItemMaster.LightItemMaster_C|SetTurnedOnByPlayer _newremotelightitem true)))))))

(fn ConstructionScript)

(fn SetTargetLocation
  (params (Int%20Pt :type Int%20Point%20Structure))
  (Variables|Default|SetTargetLocation (+ (Default|GetLocationfromGridIndex (Variables|Default|GetGrid) Int%20Pt) (Variables|Default|GetZOffset))))

(fn UpdateIndex
  (params (UpdateBy :type Int%20Point%20Structure))
  (if (Default|IsGlobalTileIndexValid (Variables|Default|GetGrid) (+ (Variables|Default|GetPlayerGridLoc) UpdateBy))
    (Variables|Default|SetPlayerGridLoc (+ (Variables|Default|GetPlayerGridLoc) UpdateBy))))

(fn MovePlayer
  (params (UpdateBy :type Int%20Point%20Structure))
  (if (Variables|Default|GetIsNotMoving)
    (CallFunction|UpdateIndex UpdateBy)
    (CallFunction|SetTargetLocation (Variables|Default|GetPlayerGridLoc))
    (Variables|Default|SetIsNotMoving false)))

(fn PickUpItem
  (bind _currentlightitem (Variables|Default|GetCurrentLightItem))
  (Utilities|IsValid _currentlightitem
    (:Is%20Valid
      (Transformation|AttachActorToActor _currentlightitem self "None" "SnapToTarget" "SnapToTarget" "SnapToTarget" true)
      (Variables|Default|SetItemEquipped true)
      (Default|PickItem _currentlightitem)
      (Development|PrintString "Item Equipped"))
    (:Is%20Not%20Valid
      (Variables|Default|SetItemEquipped false)
      (Development|PrintString "No Item here"))))

(fn DropItem
  (bind _currentlightitem (Variables|Default|GetCurrentLightItem))
  (Utilities|IsValid _currentlightitem
    (:Is%20Valid
      (if (Variables|/Game/Blueprints/Items/LightItemMaster.LightItemMaster_C|GetOnlyItemOnTile _currentlightitem)
        (Default|ItemDropped _currentlightitem (Variables|Default|GetPlayerGridLoc))
        (Variables|Default|SetItemEquipped false)
        (else
          (Development|PrintString "Multiple tiles on grid"))))
    (:Is%20Not%20Valid
      (Variables|Default|SetItemEquipped false))))

(fn DamagePlayer)