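; TestChar is a test character that tracks which GridNavMesh cell it occupies.
; The construction script caches the level's GridNavMesh, and both it and Tick update IntPt from the actor's location.
; UseEnvrionemnt selects the E or NE grid lookup for the validity check, but the stored point always comes from the NE lookup.
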(event EventBeginPlay)

(event Collision|EventActorBeginOverlap
  (params (OtherActor :type Actor%20Object%20Reference)))

(event EventTick
  (params (DeltaSeconds :type Float%20%28single-precision%29))
  (CallFunction|UpdateIntPt (Variables|Default|GetGrid)))

(fn ConstructionScript
  (Utilities|FlowControl|Sequence
    (:then_0
      (bind _returnvalue (Actor|GetActorOfClass "/Game/Blueprints/GridNavMesh.GridNavMesh_C"))
      (Utilities|IsValid _returnvalue
        (:Is%20Valid
          (bind _output_get (Variables|Default|SetGrid _returnvalue))
          (CallFunction|UpdateIntPt _output_get))))))

(fn UpdateIntPt
  (params (self2 :type Grid%20Nav%20Mesh%20Object%20Reference))
  (bind _returnvalue (Transformation|GetActorLocation))
  (bind (_isvalid _int_pt) (Default|GetGridIndexfromLocationNE self2 _returnvalue))
  (if (select (Variables|Default|GetUseEnvrionemnt) (.IsValid (Default|GetGridIndexfromLocationE self2 _returnvalue)) _isvalid)
    (Variables|Default|SetintPt _int_pt)))