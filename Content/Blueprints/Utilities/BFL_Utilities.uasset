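; Blueprint function library of tile-grid helpers for snapping, neighbor lookup and distance estimates.
; Snapping rounds each vector component to the grid's tile size, then shifts by half a tile and adds a Z offset.
; Axis, diagonal and all-neighbor queries add relative offsets to a tile index, keeping only indices the grid reports valid.
; Nearest-neighbor selection minimizes tile cost to a target, using Chebyshev distance with diagonals or Manhattan without.
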(fn SnapVectortoVector
  (params (V1 :type Vector) (V2 :type Vector))
  (return (Math|Vector|MakeVector (Math|Float|SnapToGrid(Float) (.x V1) (.x V2)) (Math|Float|SnapToGrid(Float) (.y V1) (.y V2)) (Math|Float|SnapToGrid(Float) (.z V1) (.z V2)))))

(fn SnapObjecttoGrid
  (params (Grid :type Grid%20Nav%20Mesh%20Object%20Reference) (CurrentLocation :type Vector) (ZOffset :type Float%20%28double-precision%29))
  (bind _tilesize (Variables|/Game/Blueprints/GridNavMesh.GridNavMesh_C|GetTileSize Grid))
  (bind _v3 (CallFunction|SnapVectortoVector CurrentLocation _tilesize Grid))
  (bind _returnvalue (/ _tilesize "2.000000,2.000000,2.000000"))
  (bind _returnvalue_2 (- _v3 _returnvalue))
  (return (Math|Vector|MakeVector (.x _returnvalue_2) (.y _returnvalue_2) (+ (.z _returnvalue_2) ZOffset))))

(fn GetNeighborsAlongAxes
  (params (Grid :type Grid%20Nav%20Mesh%20Object%20Reference) (Int%20Pt :type Int%20Point%20Structure))
  (for _array_element (LocalVariables|GetRelativeNeighborIndices)
    (if (Default|IsGlobalTileIndexValid Grid (+ Int%20Pt _array_element))
      (Utilities|Array|AddUnique (LocalVariables|GetAbsoluteNeightborIndices) (+ Int%20Pt _array_element))))
  (return (LocalVariables|GetAbsoluteNeightborIndices)))

(fn GetNeighborsAlongDiagonals
  (params (Grid :type Grid%20Nav%20Mesh%20Object%20Reference) (Int%20Pt :type Int%20Point%20Structure))
  (for _array_element (LocalVariables|GetRelativeNeighborIndices)
    (if (Default|IsGlobalTileIndexValid Grid (+ Int%20Pt _array_element))
      (Utilities|Array|AddUnique (LocalVariables|GetAbsoluteNeightborIndices) (+ Int%20Pt _array_element))))
  (return (LocalVariables|GetAbsoluteNeightborIndices)))

(fn GetAllNeighbors
  (params (Grid :type Grid%20Nav%20Mesh%20Object%20Reference) (Int%20Pt :type Int%20Point%20Structure))
  (for _array_element (LocalVariables|GetRelativeNeighborIndices)
    (if (Default|IsGlobalTileIndexValid Grid (+ Int%20Pt _array_element))
      (Utilities|Array|AddUnique (LocalVariables|GetAbsoluteNeightborIndices) (+ Int%20Pt _array_element))))
  (return (LocalVariables|GetAbsoluteNeightborIndices)))

(fn GetNearstNeighbortoPoint
  (params (Target :type Int%20Point%20Structure) (StartPt :type Int%20Point%20Structure) (Neighbors :type Array%20of%20Int%20Point%20Structures) (AreDiagonalsConsidered :type Boolean))
  (LocalVariables|SetMinCost (CallFunction|GetMinCostBetweenTiles StartPt Target AreDiagonalsConsidered))
  (LocalVariables|SetNearestN StartPt)
  (for _array_element Neighbors
    (if (< (CallFunction|GetMinCostBetweenTiles _array_element Target AreDiagonalsConsidered) (LocalVariables|GetMinCost))
      (LocalVariables|SetMinCost (CallFunction|GetMinCostBetweenTiles _array_element Target AreDiagonalsConsidered))
      (LocalVariables|SetNearestN _array_element)))
  (return (LocalVariables|GetNearestN)))

(fn GetMinCostBetweenTiles
  (params (StartPt :type Int%20Point%20Structure) (EndPt :type Int%20Point%20Structure) (AreDiagonalsConsidered :type Boolean))
  (bind _returnvalue (- EndPt StartPt))
  (bind _returnvalue_2 (Math|Integer|Absolute(Integer) (.x _returnvalue)))
  (bind _returnvalue_3 (Math|Integer|Absolute(Integer) (.y _returnvalue)))
  (if AreDiagonalsConsidered
    (return (Math|Integer|Max(Integer) _returnvalue_2 _returnvalue_3))
    (else
      (return (+ _returnvalue_2 _returnvalue_3)))))