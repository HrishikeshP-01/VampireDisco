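; BP_Tile_UV is a tile actor that toggles between on and off visual states.
; The construction script creates a dynamic material instance from its instanced static mesh's first material.
; TurnOn and TurnOff drive that material's SelectColor scalar parameter and record the state in IsOn.
; SwitchUV is an empty stub, and BeginPlay only calls the parent.
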(event EventBeginPlay
  (|CallParentFunction))

(event Collision|EventActorBeginOverlap
  (params (OtherActor :type Actor%20Object%20Reference))
  (|CallParentFunction OtherActor) ; This node is disabled and will not be called.\nDrag off pins to build functionality.
)

(event EventTick
  (params (DeltaSeconds :type Float%20%28single-precision%29))
  (|CallParentFunction DeltaSeconds) ; This node is disabled and will not be called.\nDrag off pins to build functionality.
)

(fn ConstructionScript
  (bind _instancedstaticmesh (Variables|Default|GetInstancedStaticMesh))
  (|CallParentFunction)
  (bind _returnvalue (Rendering|Material|CreateDynamicMaterialInstance _instancedstaticmesh 0 (Rendering|Material|GetMaterial _instancedstaticmesh 0) "None" :!class /Script/Engine.PrimitiveComponent))
  (Variables|Default|SetMaterial _returnvalue))

(fn SwitchUV)

(fn Turnon
  (Rendering|Material|SetScalarParameterValue (Variables|Default|GetMaterial) "SelectColor" 1.0 :!class /Script/Engine.MaterialInstanceDynamic)
  (Variables|Default|SetIsOn true))

(fn TurnOff
  (Rendering|Material|SetScalarParameterValue (Variables|Default|GetMaterial) "SelectColor" 0.0 :!class /Script/Engine.MaterialInstanceDynamic)
  (Variables|Default|SetIsOn false))