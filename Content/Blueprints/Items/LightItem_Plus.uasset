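; LightItem_Plus is a light item that casts beams in a plus pattern along the X and Y axes, plus one straight down.
; LightsOn stretches five spline meshes (R1 to R5) from the actor to the points returned by TraceOverTile.
; LightsOff collapses each beam to its start, then calls TraceOverTileTurnOff in the four horizontal directions to switch off connected tiles, omitting the downward one.
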(event EventBeginPlay
  (|CallParentFunction) ; This node is disabled and will not be called.\nDrag off pins to build functionality.
)

(event Collision|EventActorBeginOverlap
  (params (OtherActor :type Actor%20Object%20Reference))
  (|CallParentFunction OtherActor) ; This node is disabled and will not be called.\nDrag off pins to build functionality.
)

(event EventTick
  (params (DeltaSeconds :type Float%20%28single-precision%29))
  (|CallParentFunction DeltaSeconds) ; This node is disabled and will not be called.\nDrag off pins to build functionality.
)

(fn ConstructionScript
  (|CallParentFunction))

(fn Lightson
  (bind _r1 (Variables|Default|GetR1))
  (bind _r2 (Variables|Default|GetR2))
  (bind _r3 (Variables|Default|GetR3))
  (bind _r4 (Variables|Default|GetR4))
  (bind _r5 (Variables|Default|GetR5))
  (bind _endpoint (CallFunction|TraceOverTile "1.000000, 0, 0" 1.0))
  (SplineMesh|SetStartPosition _r1 (Transformation|GetActorLocation) true)
  (SplineMesh|SetEndPosition _r1 _endpoint true)
  (bind _endpoint_2 (CallFunction|TraceOverTile "-1.000000, 0, 0" 1.0))
  (SplineMesh|SetStartPosition _r2 (Transformation|GetActorLocation) true)
  (SplineMesh|SetEndPosition _r2 _endpoint_2 true)
  (bind _endpoint_3 (CallFunction|TraceOverTile "0,1.000000, 0" 1.0))
  (SplineMesh|SetStartPosition _r3 (Transformation|GetActorLocation) true)
  (SplineMesh|SetEndPosition _r3 _endpoint_3 true)
  (bind _endpoint_4 (CallFunction|TraceOverTile "0,-1.000000, 0" 1.0))
  (SplineMesh|SetStartPosition _r4 (Transformation|GetActorLocation) true)
  (SplineMesh|SetEndPosition _r4 _endpoint_4 true)
  (bind _endpoint_5 (CallFunction|TraceOverTile "0, 0,-1.000000" 1.0))
  (SplineMesh|SetStartPosition _r5 (Transformation|GetActorLocation) true)
  (SplineMesh|SetEndPosition _r5 _endpoint_5 true))

(fn LightsOff
  (bind _r4 (Variables|Default|GetR4))
  (bind _r3 (Variables|Default|GetR3))
  (bind _r2 (Variables|Default|GetR2))
  (bind _r5 (Variables|Default|GetR5))
  (bind _r1 (Variables|Default|GetR1))
  (SplineMesh|SetEndPosition _r4 (SplineMesh|GetStartPosition _r4) true)
  (SplineMesh|SetEndPosition _r3 (SplineMesh|GetStartPosition _r3) true)
  (SplineMesh|SetEndPosition _r2 (SplineMesh|GetStartPosition _r2) true)
  (SplineMesh|SetEndPosition _r5 (SplineMesh|GetStartPosition _r5) true)
  (SplineMesh|SetEndPosition _r1 (SplineMesh|GetStartPosition _r1) true)
  (CallFunction|InstigatorTurnConnectedTilesOff))

(fn InstigatorTurnConnectedTilesOff
  (CallFunction|TraceOverTileTurnOff (Math|Vector|MakeVector 1.0 0.0 0.0) 1.0)
  (CallFunction|TraceOverTileTurnOff (Math|Vector|MakeVector -1.0 0.0 0.0) 1.0)
  (CallFunction|TraceOverTileTurnOff (Math|Vector|MakeVector 0.0 1.0 0.0) 1.0)
  (CallFunction|TraceOverTileTurnOff (Math|Vector|MakeVector 0.0 -1.0 0.0) 1.0))