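; Light item placed over tiles that emits a diagonal cross of four beams plus one straight down.
; LightsOn runs TraceOverTile in each direction and stretches spline meshes R1 to R5 from the actor to the returned points, using a longer multiplier for diagonals.
; LightsOff calls the parent, collapses the beams, then InstigatorTurnConnectedTilesOff runs turn-off traces along the four diagonals only and prints a debug string.
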(event EventBeginPlay
  (|CallParentFunction) ; This node is disabled and will not be called.\nDrag off pins to build functionality.
)

(event Collision|EventActorBeginOverlap
  (params (OtherActor :type Actor%20Object%20Reference))
  (|CallParentFunction OtherActor) ; This node is disabled and will not be called.\nDrag off pins to build functionality.
)

(event EventTick
  (params (DeltaSeconds :type Float%20%28single-precision%29))
  (|CallParentFunction DeltaSeconds) ; This node is disabled and will not be called.\nDrag off pins to build functionality.
)

(fn ConstructionScript
  (|CallParentFunction))

(fn Lightson
  (bind _returnvalue (/ 1.0 2.0))
  (bind _r1 (Variables|Default|GetR1))
  (bind _r4 (Variables|Default|GetR4))
  (bind _r3 (Variables|Default|GetR3))
  (bind _r2 (Variables|Default|GetR2))
  (bind _r5 (Variables|Default|GetR5))
  (bind _returnvalue_2 (Math|Float|Sqrt _returnvalue))
  (bind _returnvalue_3 (* _returnvalue_2 -1.0))
  (bind _endpoint (CallFunction|TraceOverTile (Math|Vector|MakeVector _returnvalue_2 _returnvalue_2 0.0) 1.5))
  (SplineMesh|SetStartPosition _r1 (Transformation|GetActorLocation) true)
  (SplineMesh|SetEndPosition _r1 _endpoint true)
  (bind _endpoint_2 (CallFunction|TraceOverTile (Math|Vector|MakeVector _returnvalue_3 _returnvalue_3 0.0) 1.5))
  (SplineMesh|SetStartPosition _r2 (Transformation|GetActorLocation) true)
  (SplineMesh|SetEndPosition _r2 _endpoint_2 true)
  (bind _endpoint_3 (CallFunction|TraceOverTile (Math|Vector|MakeVector _returnvalue_2 _returnvalue_3 0.0) 1.5))
  (SplineMesh|SetStartPosition _r3 (Transformation|GetActorLocation) true)
  (SplineMesh|SetEndPosition _r3 _endpoint_3 true)
  (bind _endpoint_4 (CallFunction|TraceOverTile (Math|Vector|MakeVector _returnvalue_3 _returnvalue_2 0.0) 1.5))
  (SplineMesh|SetStartPosition _r4 (Transformation|GetActorLocation) true)
  (SplineMesh|SetEndPosition _r4 _endpoint_4 true)
  (bind _endpoint_5 (CallFunction|TraceOverTile "0, 0,-1.000000" 1.0))
  (SplineMesh|SetStartPosition _r5 (Transformation|GetActorLocation) true)
  (SplineMesh|SetEndPosition _r5 _endpoint_5 true))

(fn LightsOff
  (bind _r5 (Variables|Default|GetR5))
  (bind _r1 (Variables|Default|GetR1))
  (bind _r2 (Variables|Default|GetR2))
  (bind _r3 (Variables|Default|GetR3))
  (bind _r4 (Variables|Default|GetR4))
  (|CallParentFunction)
  (SplineMesh|SetEndPosition _r1 (SplineMesh|GetStartPosition _r1) true)
  (SplineMesh|SetEndPosition _r2 (SplineMesh|GetStartPosition _r2) true)
  (SplineMesh|SetEndPosition _r3 (SplineMesh|GetStartPosition _r3) true)
  (SplineMesh|SetEndPosition _r4 (SplineMesh|GetStartPosition _r4) true)
  (SplineMesh|SetEndPosition _r5 (SplineMesh|GetStartPosition _r5) true)
  (CallFunction|InstigatorTurnConnectedTilesOff))

(fn InstigatorTurnConnectedTilesOff
  (bind _returnvalue (/ 1.0 2.0))
  (bind _returnvalue_2 (Math|Float|Sqrt _returnvalue))
  (bind _returnvalue_3 (* _returnvalue_2 -1.0))
  (CallFunction|TraceOverTileTurnOff (Math|Vector|MakeVector _returnvalue_2 _returnvalue_2 0.0) 1.5)
  (CallFunction|TraceOverTileTurnOff (Math|Vector|MakeVector _returnvalue_3 _returnvalue_3 0.0) 1.5)
  (CallFunction|TraceOverTileTurnOff (Math|Vector|MakeVector _returnvalue_2 _returnvalue_3 0.0) 1.5)
  (CallFunction|TraceOverTileTurnOff (Math|Vector|MakeVector _returnvalue_3 _returnvalue_2 0.0) 1.5)
  (Development|PrintString "Tiles OFFFFF"))