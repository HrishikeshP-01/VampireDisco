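; Base actor for grid-placed light items that the player carries, drops and switches on to flash to the beat.
; GridNavMesh beats alternately call LightsOn and LightsOff while player-activated, stubs presumably overridden by children, like UseItem.
; Tile trace helpers damage players or enemies and chain neighbouring lights on or off.
; Box overlaps set the player's current and remote item, switching off the previous remote, and track tile sharing.
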(event OnComponentBeginOverlap(Box)
  (params (OverlappedComponent :type Primitive%20Component%20Object%20Reference) (OtherActor :type Actor%20Object%20Reference) (OtherComp :type Primitive%20Component%20Object%20Reference) (OtherBodyIndex :type Integer) (bFromSweep :type Boolean) (SweepResult :type Hit%20Result%20Structure%20%28by%20ref%29))
  (bind _asplayer (Utilities|Casting|CastToPlayer OtherActor)
    (:then
      (Utilities|IsValid (Variables|/Game/Blueprints/Characters/Player.Player_C|GetCurrentLightItem _asplayer)
        (:Is%20Valid
          (if (not (Variables|/Game/Blueprints/Characters/Player.Player_C|GetItemEquipped _asplayer))
            (Variables|/Game/Blueprints/Characters/Player.Player_C|SetCurrentLightItem _asplayer self)
            (Utilities|IsValid (Variables|/Game/Blueprints/Characters/Player.Player_C|GetNewRemoteLightItem _asplayer) :!label _label
              (:Is%20Valid
                (Variables|LightItemMaster_C|SetTurnedOnByPlayer (Variables|/Game/Blueprints/Characters/Player.Player_C|GetNewRemoteLightItem _asplayer) false)
                (CallFunction|LightsOff (Variables|/Game/Blueprints/Characters/Player.Player_C|GetNewRemoteLightItem _asplayer))
                (CallFunction|InstigatorTurnConnectedTilesOff (Variables|/Game/Blueprints/Characters/Player.Player_C|GetNewRemoteLightItem _asplayer)))
              (:Is%20Not%20Valid
                _))
            (Variables|/Game/Blueprints/Characters/Player.Player_C|SetNewRemoteLightItem _asplayer self)))
        (:Is%20Not%20Valid
          (Variables|/Game/Blueprints/Characters/Player.Player_C|SetCurrentLightItem _asplayer self)
          (goto _label))))
    (:CastFailed
      (Utilities|Casting|CastToLightItemMaster OtherActor)
      (Variables|Default|SetOnlyItemOnTile false))))

(event OnComponentEndOverlap(Box)
  (params (OverlappedComponent :type Primitive%20Component%20Object%20Reference) (OtherActor :type Actor%20Object%20Reference) (OtherComp :type Primitive%20Component%20Object%20Reference) (OtherBodyIndex :type Integer))
  ;[1 1 1] Make sure player overlap ends before it begins on items
  (Utilities|FlowControl|Sequence
    (:then_0
      (bind _asplayer (Utilities|Casting|CastToPlayer OtherActor))
      (if (and (not (Variables|/Game/Blueprints/Characters/Player.Player_C|GetItemEquipped _asplayer)) (Utilities|IsValid (Variables|/Game/Blueprints/Characters/Player.Player_C|GetCurrentLightItem _asplayer)))
        (Variables|/Game/Blueprints/Characters/Player.Player_C|SetCurrentLightItem _asplayer 0)
        (Development|PrintString "Item Cleared")
        (else
          (Development|PrintString "Item Not Cleared")
          (Development|PrintString (Utilities|String|ToString(Boolean) (not (Variables|/Game/Blueprints/Characters/Player.Player_C|GetItemEquipped _asplayer)))))))
    (:then_1
      (Utilities|Casting|CastToLightItemMaster OtherActor)
      (Variables|Default|SetOnlyItemOnTile true))))

(event Custom|TriggerTraceIfOn
  (if (Variables|Default|GetTurnedOnByPlayer)
    (Utilities|FlowControl|FlipFlop
      (:A
        (CallFunction|Lightson)
        (Development|PrintString "Lights Turned ON"))
      (:B
        (CallFunction|LightsOff)
        (CallFunction|InstigatorTurnConnectedTilesOff)))))

(event EventBeginPlay
  (bind _returnvalue (Actor|GetActorOfClass "/Game/Blueprints/GridNavMesh.GridNavMesh_C"))
  (bind _output_get (Variables|Default|SetGird _returnvalue))
  (EventDispatchers|BindEventtoBeatTriggered _output_get (delegate Custom|TriggerTraceIfOn)))

(event Collision|EventActorBeginOverlap
  (params (OtherActor :type Actor%20Object%20Reference)))

(event EventTick
  (params (DeltaSeconds :type Float%20%28single-precision%29)))

(fn ConstructionScript)

(fn ItemDropped
  (params (Int%20pt :type Int%20Point%20Structure))
  (bind _staticmesh (Variables|Default|GetStaticMesh))
  (bind _gird (Variables|Default|GetGird))
  (bind _loc (Default|GetLocationfromGridIndex _gird Int%20pt))
  (bind _relativelocation (Variables|/Script/Engine.SceneComponent|GetRelativeLocation _staticmesh))
  (Transformation|DetachFromActor "KeepWorld" "KeepWorld" "KeepWorld")
  (Transformation|SetActorLocation (Math|Vector|MakeVector (.x _loc) (.y _loc) (.z (Transformation|GetActorLocation))) false false)
  (Transformation|SetRelativeLocation _staticmesh (Math|Vector|MakeVector (.x _relativelocation) (.y _relativelocation) 0.0) false false))

(fn UseItem)

(fn Lightson)

(fn TraceOverTile
  (params (DirectionUnitVector :type Vector) (DiagnalOrCrossMult :type Float%20%28double-precision%29))
  (bind _returnvalue (Transformation|GetActorLocation))
  (bind _outhit (Collision|LineTraceByChannel _returnvalue (+ _returnvalue (* (* (Variables|/Game/Blueprints/GridNavMesh.GridNavMesh_C|GetTileSize (Variables|Default|GetGird)) DiagnalOrCrossMult) DirectionUnitVector)) "TraceTypeQuery4" false (Utilities|Array|MakeArray self) "ForDuration"))
  (bind _asplayer (Utilities|Casting|CastToPlayer (.HitActor (Collision|BreakHitResult _outhit)))
    (:then
      (Default|DamagePlayer _asplayer)
      (Development|PrintString "Player Hit"))
    (:CastFailed
      (bind _asenemy_master (Utilities|Casting|CastToEnemyMaster (.HitActor (Collision|BreakHitResult _outhit)))
        (:then
          (Default|Damage _asenemy_master)
          (Development|PrintString "Enemy Hit"))
        (:CastFailed
          (bind _aslight_item_master (Utilities|Casting|CastToLightItemMaster (.HitActor (Collision|BreakHitResult _outhit)))
            (:then
              (if (Variables|LightItemMaster_C|GetTurnedOn _aslight_item_master)
                _
                (else
                  (Variables|LightItemMaster_C|SetTurnedOn _aslight_item_master true)
                  (CallFunction|Lightson _aslight_item_master)
                  (Development|PrintString "Light Triggered"))))
            (:CastFailed
              _))))))
  (if (.bBlockingHit (Collision|BreakHitResult _outhit))
    (return (.Location (Collision|BreakHitResult _outhit)))
    (else
      (return (.TraceEnd (Collision|BreakHitResult _outhit))))))

(fn PickItem
  (bind _staticmesh (Variables|Default|GetStaticMesh))
  (bind _relativelocation (Variables|/Script/Engine.SceneComponent|GetRelativeLocation _staticmesh))
  (Transformation|SetRelativeLocation _staticmesh (Math|Vector|MakeVector (.x _relativelocation) (.y _relativelocation) (Variables|Default|GetZOffset)) false false))

(fn LightsOff)

(fn TraceOverTileTurnOff
  (params (DirectionUnitVector :type Vector) (DiagnalOrCrossMult :type Float%20%28double-precision%29))
  (bind _returnvalue (Transformation|GetActorLocation))
  (bind _outhit (Collision|LineTraceByChannel _returnvalue (+ _returnvalue (* (* (Variables|/Game/Blueprints/GridNavMesh.GridNavMesh_C|GetTileSize (Variables|Default|GetGird)) DiagnalOrCrossMult) DirectionUnitVector)) "TraceTypeQuery4" false (Utilities|Array|MakeArray self) "ForDuration"))
  (bind _aslight_item_master (Utilities|Casting|CastToLightItemMaster (.HitActor (Collision|BreakHitResult _outhit)))
    (:then
      (if (Variables|LightItemMaster_C|GetTurnedOn _aslight_item_master)
        (Variables|LightItemMaster_C|SetTurnedOn _aslight_item_master false)
        (CallFunction|LightsOff _aslight_item_master)
        (Development|PrintString "Light Off")
        (return)))
    (:CastFailed
      (return))))

(fn InstigatorTurnConnectedTilesOff)