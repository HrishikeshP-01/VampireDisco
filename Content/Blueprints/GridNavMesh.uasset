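; Grid actor that lays out a tile-based navigation grid as instanced static meshes, built in the construction script around its snapped location.
; With UseEnvironment on, sphere traces find BP_TileMaster actors, skipping obstacles and recording cells in global, day-night, bulb and shade arrays.
; Otherwise it fills the whole rectangle without recording cells.
; Helper functions convert between locations and grid indices, validating by bounds or recorded-tile membership.
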(event EventBeginPlay)

(event Collision|EventActorBeginOverlap
  (params (OtherActor :type Actor%20Object%20Reference)))

(event EventTick
  (params (DeltaSeconds :type Float%20%28single-precision%29)))

(fn ConstructionScript
  (Variables|Default|SetDesiredLocation (Transformation|GetActorLocation))
  (CallFunction|SpawnGrid))

(fn SpawnGrid
  (bind _tilesize (Variables|Default|GetTileSize))
  (CallFunction|ClearGrid)
  (bind (_center _corner) (CallFunction|CalculateCenterandCorner))
  (Variables|Default|SetDesiredLocation _center)
  (Variables|Default|SetGridBottomLeftCornerLoc _corner)
  (for _index (range 0 (- (.x (Variables|Default|GetTileCount)) 1))
    (LocalVariables|SetX _index)
    (for _index_2 (range 0 (- (.y (Variables|Default|GetTileCount)) 1))
      (LocalVariables|SetY _index_2)
      (LocalVariables|SetCurrentTileTransform (Math|Transform|MakeTransform (- (+ (Variables|Default|GetGridBottomLeftCornerLoc) (* _tilesize (Math|Vector|MakeVector (Math|Conversions|ToFloat(Integer) (LocalVariables|GetX)) (Math|Conversions|ToFloat(Integer) (LocalVariables|GetY)) 0.0))) (/ _tilesize "2.000000,2.000000,2.000000")) "0, 0, 0" (/ _tilesize "100.000000,100.000000,100.000000")))
      (if (Variables|Default|GetUseEnvironment)
        (bind (_tracehit _tracelocation) (CallFunction|TraceforTile (.location (LocalVariables|GetCurrentTileTransform)) (LocalVariables|GetX) (LocalVariables|GetY)))
        (if _tracehit
          (Components|InstancedStaticMesh|AddInstance (Variables|Default|GetInstancedStaticMesh) (Math|Transform|MakeTransform _tracelocation (.rotation (LocalVariables|GetCurrentTileTransform)) (.scale (LocalVariables|GetCurrentTileTransform))) true))
        (else
          (Components|InstancedStaticMesh|AddInstance (Variables|Default|GetInstancedStaticMesh) (LocalVariables|GetCurrentTileTransform) true))))))

(fn CalculateCenterandCorner
  (bind _tilecount (Variables|Default|GetTileCount))
  (bind _output_get (LocalVariables|SetNewCenter (CallFunction|SnapVectortoVector (Variables|Default|GetDesiredLocation) (Variables|Default|GetTileSize))))
  (return _output_get (- (LocalVariables|GetNewCenter) (* (Variables|Default|GetTileSize) (Math|Vector|MakeVector (Math|Conversions|ToFloat(Integer) (/ (.x _tilecount) 2)) (Math|Conversions|ToFloat(Integer) (/ (.y _tilecount) 2)) 0.0)))))

(fn TraceforTile
  (params (Location :type Vector) (X :type Integer) (Y :type Integer))
  (bind _outhits (Collision|MultiSphereTraceByChannel (+ Location "0,0,100.000000") (- Location "0,0,100.000000") (/ (.x (Variables|Default|GetTileSize)) 3.0) "TraceTypeQuery3" false 0 "ForDuration" true "(R=1.000000,G=0.000000,B=0.000000,A=1.000000)" "(R=0.000000,G=1.000000,B=0.000000,A=1.000000)" 1.0))
  (if (> (Utilities|Array|Length _outhits) 0)
    (bind _asbp_tile_master (Utilities|Casting|CastToBP_TileMaster (.HitActor (Collision|BreakHitResult (Utilities|Array|Get(acopy) _outhits)))))
    (bind _isnotobstacle (CallFunction|UpdateTileArrays _asbp_tile_master (Utilities|Struct|MakeIntPoint X Y)))
    (return _isnotobstacle (.Location (Collision|BreakHitResult (Utilities|Array|Get(acopy) _outhits))))
    (else
      (return false "-999.000000,-999.000000,-999.000000"))))

(fn UpdateTileArrays
  (params (Actor :type BP%20Tile%20Master%20Object%20Reference) (IntPt :type Int%20Point%20Structure%20%28by%20ref%29))
  (bind _tiledata (Variables|/Game/Blueprints/Tiles/BP_TileMaster.BP_TileMaster_C|GetTileData Actor))
  (if (Utilities|Enum|Equal(Enum) (.tiletype _tiledata) "NewEnumerator3")
    (return false)
    (else
      (Utilities|Array|AddUnique (Variables|TileArrays|GetGlobalTileArray) IntPt)
      (switch Utilities|FlowControl|Switch|SwitchonE_TileType (.tiletype _tiledata)
        (:NewEnumerator0
          (Utilities|Array|AddUnique (Variables|TileArrays|GetDayNightArray) IntPt))
        (:NewEnumerator1
          (Utilities|Array|AddUnique (Variables|TileArrays|GetBulbArray) IntPt))
        (:NewEnumerator2
          (Utilities|Array|AddUnique (Variables|TileArrays|GetShadeArray) IntPt)))
      (return true))))

(fn ClearGrid
  (Utilities|Array|Clear (Variables|TileArrays|GetDayNightArray))
  (Utilities|Array|Clear (Variables|TileArrays|GetBulbArray))
  (Utilities|Array|Clear (Variables|TileArrays|GetShadeArray))
  (Utilities|Array|Clear (Variables|TileArrays|GetGlobalTileArray))
  (Components|InstancedStaticMesh|ClearInstances (Variables|Default|GetInstancedStaticMesh)))

(fn GetGridIndexfromLocationNE
  (params (Loc :type Vector))
  (bind _tilesize (Variables|Default|GetTileSize))
  (bind _gridbottomleftcornerloc (Variables|Default|GetGridBottomLeftCornerLoc))
  (bind _tilesize_2 (Variables|Default|GetTileSize))
  (bind _tilecount (Variables|Default|GetTileCount))
  (bind _v3 (CallFunction|SnapVectortoVector Loc _tilesize))
  (bind _returnvalue (- _v3 _gridbottomleftcornerloc))
  (bind _returnvalue_2 (/ _returnvalue _tilesize_2))
  (bind _returnvalue_3 (Math|Float|Round (.x _returnvalue_2)))
  (bind _returnvalue_4 (Math|Float|Round (.y _returnvalue_2)))
  ;[1 1 1] Gives the index of the grid as a whole. If you want to use it make sure the tile exists by doing something like a line trace first
  (return (and (Math|Integer|InRange(Integer) _returnvalue_3 0 (- (.x _tilecount) 1)) (Math|Integer|InRange(Integer) _returnvalue_4 0 (- (.y _tilecount) 1))) (Utilities|Struct|MakeIntPoint _returnvalue_3 _returnvalue_4)))

(fn GetGridIndexfromLocationE
  (params (Loc :type Vector))
  (bind _tilesize (Variables|Default|GetTileSize))
  (bind _gridbottomleftcornerloc (Variables|Default|GetGridBottomLeftCornerLoc))
  (bind _tilesize_2 (Variables|Default|GetTileSize))
  (bind _v3 (CallFunction|SnapVectortoVector Loc _tilesize))
  (bind _returnvalue (- _v3 _gridbottomleftcornerloc))
  (bind _returnvalue_2 (/ _returnvalue _tilesize_2))
  (bind _returnvalue_3 (Math|Float|Round (.x _returnvalue_2)))
  (bind _returnvalue_4 (Math|Float|Round (.y _returnvalue_2)))
  (bind _intpoint (Utilities|Struct|MakeIntPoint _returnvalue_3 _returnvalue_4))
  (return (Utilities|Array|ContainsItem (Variables|TileArrays|GetGlobalTileArray) _intpoint) _intpoint))

(fn IsGlobalTileIndexValid
  (params (Int%20Pt :type Int%20Point%20Structure))
  (if (Utilities|Array|ContainsItem (Variables|TileArrays|GetGlobalTileArray) Int%20Pt)
    (return true)
    (else
      (return false))))

(fn GetLocationfromGridIndex
  (params (Int%20Pt :type Int%20Point%20Structure))
  (bind _tilesize (Variables|Default|GetTileSize))
  (return (- (+ (Variables|Default|GetGridBottomLeftCornerLoc) (* _tilesize (Math|Vector|MakeVector (Math|Conversions|ToFloat(Integer) (.x Int%20Pt)) (Math|Conversions|ToFloat(Integer) (.y Int%20Pt)) 0.0))) (/ _tilesize "2.000000,2.000000,2.000000"))))