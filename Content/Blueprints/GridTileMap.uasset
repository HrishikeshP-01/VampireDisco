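; GridTileMap is an actor that builds a flat grid of tiles as instances on one InstancedStaticMesh, rebuilt in the construction script.
; The actor's location is snapped to the tile size to get the grid center, from which the bottom-left corner is derived.
; SpawnGrid clears old instances, then loops over TileCount to add world-space tiles scaled by TileSize / 100.
; The event graph holds no runtime logic.
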(event EventBeginPlay)

(event Collision|EventActorBeginOverlap
  (params (OtherActor :type Actor%20Object%20Reference)))

(event EventTick
  (params (DeltaSeconds :type Float%20%28single-precision%29)))

(fn ConstructionScript
  (Variables|Default|SetDesiredLocation (Transformation|GetActorLocation))
  (CallFunction|SpawnGrid))

(fn SpawnGrid
  (bind _tilesize (Variables|Default|GetTileSize))
  (Components|InstancedStaticMesh|ClearInstances (Variables|Default|GetInstancedStaticMesh))
  (bind (_center _corner) (CallFunction|CalculateCenterandCorner))
  (Variables|Default|SetDesiredLocation _center)
  (Variables|Default|SetGridBottomLeftCornerLoc _corner)
  (for _index (range 0 (- (.x (Variables|Default|GetTileCount)) 1))
    (LocalVariables|SetX _index)
    (for _index_2 (range 0 (- (.y (Variables|Default|GetTileCount)) 1))
      (LocalVariables|SetY _index_2)
      (bind _output_get (LocalVariables|SetCurrentTileTransform (Math|Transform|MakeTransform (- (+ (Variables|Default|GetGridBottomLeftCornerLoc) (* _tilesize (Math|Vector|MakeVector (Math|Conversions|ToFloat(Integer) (LocalVariables|GetX)) (Math|Conversions|ToFloat(Integer) (LocalVariables|GetY)) 0.0))) (/ _tilesize "2.000000,2.000000,2.000000")) "0, 0, 0" (/ _tilesize "100.000000,100.000000,100.000000"))))
      (Components|InstancedStaticMesh|AddInstance (Variables|Default|GetInstancedStaticMesh) _output_get true))))

(fn CalculateCenterandCorner
  (bind _tilecount (Variables|Default|GetTileCount))
  (bind _output_get (LocalVariables|SetNewCenter (CallFunction|SnapVectortoVector (Variables|Default|GetDesiredLocation) (Variables|Default|GetTileSize))))
  (return _output_get (- (LocalVariables|GetNewCenter) (* (Variables|Default|GetTileSize) (Math|Vector|MakeVector (Math|Conversions|ToFloat(Integer) (/ (.x _tilecount) 2)) (Math|Conversions|ToFloat(Integer) (/ (.y _tilecount) 2)) 0.0)))))