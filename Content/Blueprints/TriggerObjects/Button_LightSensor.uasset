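; Light sensor button Blueprint that holds an on/off Activated state and shows it through material glow.
; The construction script creates a dynamic material instance on the static mesh's second material slot and tints it with the Color variable.
; TurnOn and TurnOff set Activated and raise or lower the material's Emission.
; The event graph is empty, so the file contains no detection logic of its own.
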(event EventBeginPlay
  (|CallParentFunction) ; This node is disabled and will not be called.\nDrag off pins to build functionality.
)

(event Collision|EventActorBeginOverlap
  (params (OtherActor :type Actor%20Object%20Reference))
  (|CallParentFunction OtherActor) ; This node is disabled and will not be called.\nDrag off pins to build functionality.
)

(event EventTick
  (params (DeltaSeconds :type Float%20%28single-precision%29))
  (|CallParentFunction DeltaSeconds) ; This node is disabled and will not be called.\nDrag off pins to build functionality.
)

(fn ConstructionScript
  (bind _staticmesh (Variables|Default|GetStaticMesh))
  (|CallParentFunction)
  (bind _returnvalue (Rendering|Material|CreateDynamicMaterialInstance _staticmesh 1 (Rendering|Material|GetMaterial _staticmesh 1) "None" :!class /Script/Engine.PrimitiveComponent))
  (bind _output_get (Variables|Default|SetMaterial _returnvalue))
  (Rendering|Material|SetVectorParameterValue _output_get "Color" (Variables|Default|GetColor) :!class /Script/Engine.MaterialInstanceDynamic))

(fn Turnon
  (Rendering|Material|SetScalarParameterValue (Variables|Default|GetMaterial) "Emission" 3.0 :!class /Script/Engine.MaterialInstanceDynamic)
  (Variables|Default|SetActivated true))

(fn TurnOff
  (Rendering|Material|SetScalarParameterValue (Variables|Default|GetMaterial) "Emission" 1.0 :!class /Script/Engine.MaterialInstanceDynamic)
  (Variables|Default|SetActivated false))